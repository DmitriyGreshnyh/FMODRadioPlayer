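; Player music component that runs an in-game radio with three modes: city radio, user music and online radio, starting in city mode.
; A state switch routes playback, skipping and data refresh to the track or station logic, with shuffle, repeat and change notifications.
; FMOD programmer sounds play track paths and stream URLs through ambient-sound actor components, while city radio creates its own component on the owner.
; Pausing affects only city radio.
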(event `self.ReceiveBeginPlay`
  (`self.UpdateTrackList`)
  (`self.LoadStations`)
  (`self.ChangeRadioState` "NewEnumerator0")
  ;[1 1 1] Менять компоненты FMOD после смены машины. принудительно выключая радио
  (add `Controller.OnPossessedPawnChanged` (`GameplayStatics.GetPlayerController` 0) (delegate `OnPossessedPawnChanged_Event`)))

(event `OnPossessedPawnChanged_Event`
  (params (OldPawn :type "Pawn Object Reference") (NewPawn :type "Pawn Object Reference"))
  ;[1 1 1] Менять компоненты FMOD после смены машины. принудительно выключая радио
)

(fn `ChangeRadioState`
  (params (NewState :type "/FMODRadioPlayer/E_MusicPlayerState Enum" :default "NewEnumerator0"))
  (`self.StopMusic`)
  (set `self.CurState` NewState))

(fn `DeleteStation`
  (params (Station :type "RadioStation Structure"))
  (if (== Station (`self.GetCurrentStation`))
    (if (`self.IsOnlineRadioPlaying`)
      (`self.StopMusic`))
    (`self.RemoveRadioStation` (`local.Station`))
    (`self.OnStationSelected` (`self.GetCurrentStation`))
    (else
      (`self.RemoveRadioStation` (`local.Station`)))))

(fn `GetCityRadioComponent`
  (returns (Output_Get :type "FMODAudioComponent Object Reference"))
  (`self.FME_CityRadio`
    (:`then`
      (return (`self.FME_CityRadio`)))
    (:`else`
      (bind _returnvalue (`|AddComponentByClass` :`self` (`self.GetOwner`) :`Class` "/Script/FMODStudio.FMODAudioComponent"))
      (`FMODAudioComponent.SetEvent` _returnvalue "/Game/FMOD/Events/FME_CityRadio.FME_CityRadio")
      (bind _output_get (set `self.FME_CityRadio` _returnvalue))
      (return _output_get))))

(fn `GetCurrentState`
  (returns (CurState :type "/FMODRadioPlayer/E_MusicPlayerState Enum"))
  (return (`self.CurState`)))

(fn `GetCurrentStation`
  (returns (CurStation :type "RadioStation Structure"))
  (if (not (`self.IsStationSelected`))
    (`self.SelectStation` (`|GetArrayItem` (`self.GetRadioStations`)))
    (return (`self.CurStation`))
    (else
      (return (`self.CurStation`)))))

(fn `GetCurrentTrack`
  (returns (CurTrack :type "MusicMeta Structure"))
  (locals (LocTrack :type "MusicMeta Structure"))
  (if (not (`self.IsTrackSelected`))
    (if (`self.bTracksShuffled`)
      (set `local.LocTrack` (`|GetArrayItem` (`self.GetShuffledTracks`)))
      (else
        (set `local.LocTrack` (`|GetArrayItem` (`self.GetTrackList`)))))
    (`self.SelectTrack` (`local.LocTrack`))
    (return (`self.CurTrack`))
    (else
      (return (`self.CurTrack`)))))

(fn `GetOnlineRadioComponent`
  (returns (Output_Get :type "FMODAudioComponent Object Reference"))
  (`self.FME_OnlinerRadio`
    (:`then`
      (return (`self.FME_OnlinerRadio`)))
    (:`else`
      (bind _returnvalue (`GameplayStatics.GetActorOfClass` "/Script/FMODStudio.FMODAmbientSound"))
      (bind _output_get (set `self.FME_OnlinerRadio` (`FMODAmbientSound.AudioComponent` _returnvalue)))
      (return _output_get))))

(fn `GetShuffledTracks`
  (returns (ShuffledTracks :type "Array of MusicMeta Structure"))
  (return (`self.TracksShuffled`)))

(fn `GetUserRadioComponent`
  (returns (Output_Get :type "FMODAudioComponent Object Reference"))
  (`self.FME_UserRadio`
    (:`then`
      (return (`self.FME_UserRadio`)))
    (:`else`
      (bind _returnvalue (`GameplayStatics.GetActorOfClass` "/Script/FMODStudio.FMODAmbientSound"))
      (bind _output_get (set `self.FME_UserRadio` (`FMODAmbientSound.AudioComponent` _returnvalue)))
      (return _output_get))))

(fn `IsCityRadioPlaying`
  (returns (Playing :type Boolean))
  (return (`self.bCityRadioPlaying`)))

(fn `IsMusicPaused`
  (returns (bMusicPaused :type Boolean))
  (return (`self.bMusicPaused`)))

(fn `IsMusicPlaying`
  (returns (Playing :type Boolean))
  (if (`self.IsUserMusicPlaying`)
    (return true)
    (elif (`self.IsOnlineRadioPlaying`)
      (return true)
      (else
        (return (`self.IsCityRadioPlaying`))))))

(fn `IsOnlineRadioPlaying`
  (returns (Playing :type Boolean))
  (return (`self.bOnlineRadioPlaying`)))

(fn `IsStationSelected`
  (returns (ReturnValue :type Boolean))
  (bind (_curstation_name _curstation_url) (break `RadioStation` (`self.CurStation`)))
  (return (not (and (`KismetStringLibrary.IsEmpty` _curstation_name) (`KismetStringLibrary.IsEmpty` _curstation_url)))))

(fn `IsTrackRepeating`
  (returns (bTrackRepeat :type Boolean))
  (return (`self.bTrackRepeat`)))

(fn `IsTrackSelected`
  (returns (ReturnValue :type Boolean))
  (locals (NewLocalVar :type "MusicMeta Structure"))
  (bind (_curtrack_name _curtrack_path) (break `MusicMeta` (`self.CurTrack`)))
  (return (not (`KismetStringLibrary.IsEmpty` _curtrack_path))))

(fn `IsTracksShuffled`
  (returns (bTracksShuffled :type Boolean))
  (return (`self.bTracksShuffled`)))

(fn `IsUserMusicPlaying`
  (returns (Playing :type Boolean))
  (return (`self.bUserMusicPlaying`)))

(fn `Next`
  (`self.StateSwitch`
    (:`UserMusic`
      (`self.NextTrack`))
    (:`OnlineRadio`
      (`self.NextOnlineStation`))))

(fn `NextOnlineStation`
  (locals (LocStationsOld :type "Array of  Structure") (LocCurIndex :type Integer :default 0) (LocStations :type "Array of RadioStation Structure"))
  (set `local.LocStations` (`self.GetRadioStations`))
  (set `local.LocCurIndex` (`KismetArrayLibrary.Array_Find` (`local.LocStations`) (`self.GetCurrentStation`)))
  (`self.SelectStation` (select `bool` (== (`local.LocCurIndex`) (`KismetArrayLibrary.Array_LastIndex` (`local.LocStations`))) :`false` (`|GetArrayItem` (`local.LocStations`) (+ (`local.LocCurIndex`) 1)) :`true` (`|GetArrayItem` (`local.LocStations`))))
  (if (`self.IsOnlineRadioPlaying`)
    (`self.PlayOnlineRadio`)))

(fn `NextTrack`
  (locals (LocCurIndex :type Integer :default 0) (LocTrackList :type "Array of MusicMeta Structure"))
  (if (not (`self.IsTrackRepeating`))
    (if (`self.bTracksShuffled`)
      (set `local.LocTrackList` (`self.GetShuffledTracks`))
      (else
        (set `local.LocTrackList` (`self.GetTrackList`))))
    (set `local.LocCurIndex` (`KismetArrayLibrary.Array_Find` (`local.LocTrackList`) (`self.GetCurrentTrack`)))
    (`self.SelectTrack` (select `bool` (== (`local.LocCurIndex`) (`KismetArrayLibrary.Array_LastIndex` (`local.LocTrackList`))) :`false` (`|GetArrayItem` (`local.LocTrackList`) (+ (`local.LocCurIndex`) 1)) :`true` (`|GetArrayItem` (`local.LocTrackList`))))
    (else
      (`self.SelectTrack` (`self.GetCurrentTrack`)))))

(fn `OnOnlineRadioStoppped`)

(fn `PauseMusic`
  (`FMODAudioComponent.SetPaused` (`self.GetCityRadioComponent`) true)
  (set `self.bMusicPaused` true)
  (`self.OnPlayerButtonsChanged`))

(fn `PlayCityRadio`
  (if (`self.bCityRadioPlaying`)
    (if (`self.bMusicPaused`)
      (`FMODAudioComponent.SetPaused` (`self.GetCityRadioComponent`) false)
      (set `self.bMusicPaused` false))
    (else
      (`FMODAudioComponent.Play` (`self.GetCityRadioComponent`))
      (set `self.bCityRadioPlaying` true))))

(fn `PlayMusic`
  (`self.StateSwitch`
    (:`CityRadio`
      (`self.PlayCityRadio`))
    (:`UserMusic`
      (`self.PlayUserMusic`))
    (:`OnlineRadio`
      (`self.PlayOnlineRadio`)))
  (`self.OnPlayerButtonsChanged`))

(fn `PlayOnlineRadio`
  (`FMODAudioComponent.SetProgrammerSoundName` (`self.GetOnlineRadioComponent`) (`.Url` (break `RadioStation` (`self.GetCurrentStation`))))
  (`FMODAudioComponent.Play` (`self.GetOnlineRadioComponent`))
  (add `FMODAudioComponent.OnEventStopped` (`self.GetOnlineRadioComponent`) (`|CreateDelegate` :!event `OnOnlineRadioStoppped`))
  (set `self.bOnlineRadioPlaying` true))

(fn `PlayUserMusic`
  (bind _returnvalue (`FMODAudioComponent.GetPaused` (`self.GetUserRadioComponent`)))
  (if _returnvalue
    (`FMODAudioComponent.SetPaused` (`self.GetUserRadioComponent`) false)
    (else
      (`FMODAudioComponent.SetProgrammerSoundName` (`self.GetUserRadioComponent`) (`.Path` (break `MusicMeta` (`self.GetCurrentTrack`))))
      (`FMODAudioComponent.Play` (`self.GetUserRadioComponent`))))
  (add `FMODAudioComponent.OnEventStopped` (`self.GetUserRadioComponent`) (`|CreateDelegate` :!event `NextTrack`))
  (set `self.bUserMusicPlaying` true))

(fn `Previous`
  (`self.StateSwitch`
    (:`UserMusic`
      (`self.PreviousTrack`))
    (:`OnlineRadio`
      (`self.PreviousOnlineStation`))))

(fn `PreviousOnlineStation`
  (locals (LocStationsOld :type "Array of  Structure") (LocCurIndex :type Integer :default 0) (LocStations :type "Array of RadioStation Structure"))
  (set `local.LocStations` (`self.GetRadioStations`))
  (set `local.LocCurIndex` (`KismetArrayLibrary.Array_Find` (`local.LocStations`) (`self.GetCurrentStation`)))
  (`self.SelectStation` (select `bool` (== (`local.LocCurIndex`) 0) :`false` (`|GetArrayItem` (`local.LocStations`) (- (`local.LocCurIndex`) 1)) :`true` (`|GetArrayItem` (`local.LocStations`) (`KismetArrayLibrary.Array_LastIndex` (`local.LocStations`)))))
  (if (`self.IsOnlineRadioPlaying`)
    (`self.PlayOnlineRadio`)))

(fn `PreviousTrack`
  (locals (LocTrackListOld :type "Array of  Structure") (LocCurIndex :type Integer :default 0) (LocTrackList :type "Array of MusicMeta Structure"))
  (if (`self.bTracksShuffled`)
    (set `local.LocTrackList` (`self.GetShuffledTracks`))
    (else
      (set `local.LocTrackList` (`self.GetTrackList`))))
  (set `local.LocCurIndex` (`KismetArrayLibrary.Array_Find` (`local.LocTrackList`) (`self.GetCurrentTrack`)))
  (`self.SelectTrack` (select `bool` (== (`local.LocCurIndex`) 0) :`false` (`|GetArrayItem` (`local.LocTrackList`) (- (`local.LocCurIndex`) 1)) :`true` (`|GetArrayItem` (`local.LocTrackList`) (`KismetArrayLibrary.Array_LastIndex` (`local.LocTrackList`)))))
  (if (`self.IsUserMusicPlaying`)
    (`self.PlayUserMusic`)))

(fn `SelectStation`
  (params (Station :type "RadioStation Structure"))
  (bind _output_get (set `self.CurStation` Station))
  (`self.OnStationSelected` _output_get)
  (if (`self.bOnlineRadioPlaying`)
    (`self.StopMusic`)
    (`self.PlayOnlineRadio`)))

(fn `SelectTrack`
  (params (Track :type "MusicMeta Structure"))
  (bind _output_get (set `self.CurTrack` Track))
  (`self.OnTrackSelected` _output_get)
  (`self.StateSwitch`
    (:`UserMusic`
      (if (`self.bUserMusicPlaying`)
        (`self.StopMusic`)
        (`self.PlayMusic`)))))

(fn `SetTrackRepeat`
  (params (TrackRepeat :type Boolean))
  (set `self.bTrackRepeat` TrackRepeat)
  (`self.OnPlayerButtonsChanged`))

(fn `SetTracksShuffled`
  (params (bShuffled :type Boolean))
  (if bShuffled
    (bind _output_get (set `self.TracksShuffled` (`self.GetTrackList`)))
    (`KismetArrayLibrary.Array_Shuffle` _output_get)
    (set `self.bTracksShuffled` true)
    (else
      (set `self.bTracksShuffled` false)
      (`KismetArrayLibrary.Array_Clear` (`self.TracksShuffled`))))
  (`self.OnPlayerButtonsChanged`)
  (`self.OnTracksShuffelingChanged` (`self.bTracksShuffled`)))

(fn `StopMusic`
  (remove `FMODAudioComponent.OnEventStopped` (`self.GetUserRadioComponent`) (`|CreateDelegate` :!event `NextTrack`))
  (`FMODAudioComponent.Stop` (`self.GetUserRadioComponent`))
  (`FMODAudioComponent.Stop` (`self.GetOnlineRadioComponent`))
  (`FMODAudioComponent.Stop` (`self.GetCityRadioComponent`))
  (set `self.bUserMusicPlaying` false)
  (set `self.bOnlineRadioPlaying` false)
  (set `self.bCityRadioPlaying` false)
  (`self.OnPlayerButtonsChanged`))

(fn `UpdateData`
  (`self.StateSwitch`
    (:`UserMusic`
      (`self.UpdateTrackList`))
    (:`OnlineRadio`
      (`self.LoadStations`))))